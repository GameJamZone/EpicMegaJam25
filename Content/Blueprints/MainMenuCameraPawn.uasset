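; Main menu camera pawn that flies along a referenced spline after being possessed by the first player controller at BeginPlay.
; A timeline, with its play rate set to the inverse of TimeToComplete, drives an alpha along the spline's length.
; Each update sets the pawn's world location and rotation from the spline at that distance, so the view follows the path's direction.
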(event Custom|MoveObject
  (bind _splineref (Variables|Default|GetSplineRef))
  (bind _spline (Variables|/Game/HereWeGoAgain/Actors/BP_CarSplinePath.BP_CarSplinePath_C|GetSpline _splineref))
  (Components|Timeline|SetPlayRate (Variables|Default|GetT_Move) (/ 1.0 (Variables|Default|GetTimeToComplete)))
  (bind _movetrack (Timeline|T_Move Play)
    (:Update
      (Transformation|SetActorLocationAndRotation (Spline|GetLocationatDistanceAlongSpline _spline (Math|Float|Lerp 0.0 (Spline|GetSplineLength _spline) _movetrack) "World") (Spline|GetRotationatDistanceAlongSpline _spline (Math|Float|Lerp 0.0 (Spline|GetSplineLength _spline) _movetrack) "World")))))

(event EventBeginPlay
  (CallFunction|MoveObject)
  (Pawn|Possess (Game|GetPlayerController 0) self))

(event Collision|EventActorBeginOverlap
  (params (OtherActor :type Actor%20Object%20Reference)))

(event EventTick
  (params (DeltaSeconds :type Float%20%28single-precision%29)))

(fn ConstructionScript)