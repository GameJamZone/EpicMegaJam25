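; BP_Boss is an enemy boss character that turns to face the player.
; Each tick it eases toward the look-at rotation to the first player character with a fixed-alpha lerp, keeping its own pitch and applying the interpolated yaw and roll.
; On any actor overlap it disables movement, then immediately switches its movement mode to Flying.
; BeginPlay and the construction script are empty.
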(event EventBeginPlay)

(event Collision|EventActorBeginOverlap
  (params (OtherActor :type Actor%20Object%20Reference))
  (bind _charactermovement (Variables|Character|GetCharacterMovement))
  (Pawn|Components|CharacterMovement|DisableMovement _charactermovement)
  (Pawn|Components|CharacterMovement|SetMovementMode _charactermovement "MOVE_Flying" 0))

(event EventTick
  (params (DeltaSeconds :type Float%20%28single-precision%29))
  (bind _returnvalue (Game|GetPlayerCharacter 0))
  (bind _returnvalue_2 (Transformation|GetActorLocation))
  (bind _returnvalue_3 (Transformation|GetActorRotation))
  (bind _returnvalue_4 (Transformation|GetActorLocation _returnvalue))
  (bind _returnvalue_5 (Math|Rotator|FindLookatRotation _returnvalue_2 _returnvalue_4))
  (bind _returnvalue_6 (Math|Rotator|Lerp(Rotator) _returnvalue_3 _returnvalue_5 0.05 true))
  (Transformation|SetActorRotation (Math|Rotator|MakeRotator (.roll _returnvalue_6) (.Pitch (Math|Rotator|BreakRotator _returnvalue_3)) (.yaw _returnvalue_6))))

(fn ConstructionScript)